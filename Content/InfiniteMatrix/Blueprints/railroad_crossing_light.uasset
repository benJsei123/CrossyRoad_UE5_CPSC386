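; Railroad crossing signal actor with two lights that flash alternately when triggered.
; Each Tick checks the IsBlinking flag, clears it and plays a timeline from the start.
; The timeline's blinking track toggles visibility between the left and right lights around a midpoint threshold, and both lights are hidden when it finishes.
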(event EventBeginPlay)

(event Collision|EventActorBeginOverlap
  (params (OtherActor :type Actor%20Object%20Reference)))

(event EventTick
  (params (DeltaSeconds :type Float%20%28single-precision%29))
  (if (== (Variables|Default|GetisBlinking) true)
    (Variables|Default|SetisBlinking false)
    (bind _blinkingtrack (Timeline|Timeline PlayFromStart)
      (:Update
        (if (> _blinkingtrack 0.5)
          (Rendering|SetVisibility (Variables|Default|GetLeftLight) false false)
          (Rendering|SetVisibility (Variables|Default|GetRIght%20Light1) true false)
          (else
            (Rendering|SetVisibility (Variables|Default|GetRIght%20Light1) false false)
            (Rendering|SetVisibility (Variables|Default|GetLeftLight) true false))))
      (:Finished
        (Rendering|SetVisibility (Variables|Default|GetLeftLight) false false)
        (Rendering|SetVisibility (Variables|Default|GetRIght%20Light1) false false)))))

(fn ConstructionScript)