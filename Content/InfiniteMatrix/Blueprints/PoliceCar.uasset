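; Police car actor that moves by projectile movement and spins its red and blue roof lights.
; Tick advances the yaw of both lights by LightRotationSpeed each frame.
; When its Box begins overlapping a Vehicle or another PoliceCar, it sets both cars' max and initial projectile speeds to the same low value.
; Overlapping any other actor sets its own speeds to a higher value.
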(event OnComponentBeginOverlap(Box)
  (params (OverlappedComponent :type Primitive%20Component%20Object%20Reference) (OtherActor :type Actor%20Object%20Reference) (OtherComp :type Primitive%20Component%20Object%20Reference) (OtherBodyIndex :type Integer) (bFromSweep :type Boolean) (SweepResult :type Hit%20Result%20Structure%20%28by%20ref%29))
  (bind _asvehicle (Utilities|Casting|CastToVehicle OtherActor)
    (:then
      ;[1 1 1] Decrease own speed (police car
      (bind _output_get (Variables|Default|SetProjectileMovement (Variables|Default|GetProjectileMovement)))
      (Variables|/Script/Engine.ProjectileMovementComponent|SetMaxSpeed _output_get 2e+02)
      (Variables|/Script/Engine.ProjectileMovementComponent|SetInitialSpeed _output_get 2e+02)
      ;[1 1 1] equal hit vehicl's speed
      (bind _output_get_2 (Variables|/Game/InfiniteMatrix/Blueprints/Vehicle.Vehicle_C|SetProjectileMovement _asvehicle (Variables|/Game/InfiniteMatrix/Blueprints/Vehicle.Vehicle_C|GetProjectileMovement _asvehicle)))
      (Variables|/Script/Engine.ProjectileMovementComponent|SetMaxSpeed _output_get_2 2e+02)
      (Variables|/Script/Engine.ProjectileMovementComponent|SetInitialSpeed _output_get_2 2e+02))
    (:CastFailed
      (bind _aspolice_car (Utilities|Casting|CastToPoliceCar OtherActor)
        (:then
          ;[1 1 1] Decrease own speed (police car
          (bind _output_get_3 (Variables|Default|SetProjectileMovement (Variables|Default|GetProjectileMovement)))
          (Variables|/Script/Engine.ProjectileMovementComponent|SetMaxSpeed _output_get_3 2e+02)
          (Variables|/Script/Engine.ProjectileMovementComponent|SetInitialSpeed _output_get_3 2e+02)
          ;[1 1 1] Inrease hit police car"s speed
          (Variables|/Script/Engine.ProjectileMovementComponent|SetMaxSpeed (Variables|PoliceCar_C|GetProjectileMovement _aspolice_car) 2e+02)
          (Variables|/Script/Engine.ProjectileMovementComponent|SetInitialSpeed (Variables|PoliceCar_C|GetProjectileMovement _aspolice_car) 2e+02))
        (:CastFailed
          (bind _output_get_4 (Variables|Default|SetProjectileMovement (Variables|Default|GetProjectileMovement)))
          (Variables|/Script/Engine.ProjectileMovementComponent|SetInitialSpeed _output_get_4 6e+02)
          (Variables|/Script/Engine.ProjectileMovementComponent|SetMaxSpeed _output_get_4 6e+02))))))

(event EventTick
  (params (DeltaSeconds :type Float%20%28single-precision%29))
  (bind _rightlightred (Variables|Default|GetRightLightRed))
  (bind _leftlightblue (Variables|Default|GetLeftLightBlue))
  (bind _returnvalue (Transformation|GetWorldRotation _rightlightred))
  (bind _returnvalue_2 (Transformation|GetWorldRotation _leftlightblue))
  (Transformation|SetWorldRotation (Variables|Default|GetRightLightRed) (Math|Rotator|MakeRotator (.roll _returnvalue) (.pitch _returnvalue) (+ (.yaw _returnvalue) (Variables|Default|GetLightRotationSpeed))) false false)
  (Transformation|SetWorldRotation (Variables|Default|GetLeftLightBlue) (Math|Rotator|MakeRotator (.roll _returnvalue_2) (.pitch _returnvalue_2) (+ (.yaw _returnvalue_2) (Variables|Default|GetLightRotationSpeed))) false false))

(fn ConstructionScript)