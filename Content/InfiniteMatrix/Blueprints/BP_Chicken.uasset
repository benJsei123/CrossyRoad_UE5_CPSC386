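; Player chicken character for a Crossy Road-style game, hopping across lanes of traffic, trains and water.
; Axis input launches grounded hops, sized by the current lane when moving forward or back, while timelines turn the mesh.
; A backward-hop counter drives Eagle spawning, and the Cleaner component destroys actors it overlaps.
; Capsule overlaps handle deaths by squashing, drowning or eagle (detaching the camera), then set GameOver and show the restart widget.
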(event OnComponentBeginOverlap(Cleaner)
  (params (OverlappedComponent :type Primitive%20Component%20Object%20Reference) (OtherActor :type Actor%20Object%20Reference) (OtherComp :type Primitive%20Component%20Object%20Reference) (OtherBodyIndex :type Integer) (bFromSweep :type Boolean) (SweepResult :type Hit%20Result%20Structure%20%28by%20ref%29))
  (Actor|DestroyActor OtherActor))

(event OnComponentBeginOverlap(CapsuleComponent)
  (params (OverlappedComponent :type Primitive%20Component%20Object%20Reference) (OtherActor :type Actor%20Object%20Reference) (OtherComp :type Primitive%20Component%20Object%20Reference) (OtherBodyIndex :type Integer) (bFromSweep :type Boolean) (SweepResult :type Hit%20Result%20Structure%20%28by%20ref%29))
  (bind _chicken (Variables|Default|GetChicken))
  (bind _chicken_2 (Variables|Default|GetChicken))
  (bind _chicken_3 (Variables|Default|GetChicken))
  (bind _returnvalue (Transformation|GetWorldLocation _chicken_3))
  (bind _returnvalue_2 (Transformation|GetWorldLocation _chicken_2))
  (bind _relativescale3d (Variables|/Script/Engine.SceneComponent|GetRelativeScale3D _chicken))
  (bind (_x _y) (Math|Vector|BreakVector _relativescale3d))
  (Utilities|Casting|CastToVehicle OtherActor
    (:then
      (Transformation|SetRelativeScale3D _chicken (Math|Vector|MakeVector _x _y 0.001) :!label _label)
      (Collision|SetCollisionEnabled (Variables|Collision|GetCapsuleComponent) "NoCollision")
      ;[1 1 1] Make chicke n land on ground, then disable further movement
      (bind _newtrack_0 (Timeline|Timeline_3 PlayFromStart)
        (:Update
          (Transformation|SetWorldLocation _chicken_2 (Math|Vector|MakeVector (.x _returnvalue_2) (.y _returnvalue_2) (.z (Math|Vector|Lerp(Vector) (Math|Vector|MakeVector 0.0 0.0 (.z _returnvalue_2)) (Math|Vector|MakeVector 0.0 0.0 3e+01) _newtrack_0))) false false))
        (:Finished
          (Physics|SetSimulatePhysics (Variables|Default|GetChicken) false)
          (Pawn|Components|CharacterMovement|DisableMovement (Variables|Character|GetCharacterMovement))))
      (Variables|Default|SetgameOver true)
      (bind _returnvalue_3 (UserInterface|CreateWidget "/Game/InfiniteMatrix/Blueprints/RestartButton.RestartButton_C"))
      (bind _output_get (Variables|Default|SetRestartButton_UI _returnvalue_3))
      (UserInterface|Viewport|AddtoViewport _output_get 0)
      (Variables|/Script/Engine.PlayerController|SetbShowMouseCursor (Game|GetPlayerController 0) true))
    (:CastFailed
      (Utilities|Casting|CastToTrain OtherActor
        (:then
          (goto _label))
        (:CastFailed
          (Utilities|Casting|CastToPoliceCar OtherActor
            (:then
              (goto _label))
            (:CastFailed
              (bind _asbp_lane (Utilities|Casting|CastToBP_Lane OtherActor)
                (:then
                  (if (Math|Boolean|ANDBoolean (== (Variables|/Game/InfiniteMatrix/Blueprints/BP_Lane.BP_Lane_C|GetisWater _asbp_lane) true) (== (Variables|Default|GetisOnLog) false) (<= (.z (Transformation|GetWorldLocation (Variables|Default|GetChicken))) 4e+01))
                    (Collision|SetCollisionEnabled (Variables|Collision|GetCapsuleComponent) "NoCollision")
                    ;[1 1 1] Make chicke n land on ground, then disable further movement
                    (bind _newtrack_0_2 (Timeline|Timeline_4 PlayFromStart)
                      (:Update
                        (Transformation|SetWorldLocation _chicken_3 (Math|Vector|MakeVector (.x _returnvalue) (.y _returnvalue) (.z (Math|Vector|Lerp(Vector) (Math|Vector|MakeVector 0.0 0.0 (.z _returnvalue)) (Math|Vector|MakeVector 0.0 0.0 -5e+01) _newtrack_0_2))) false false))
                      (:Finished
                        (Physics|SetSimulatePhysics (Variables|Default|GetChicken) false)
                        (Pawn|Components|CharacterMovement|DisableMovement (Variables|Character|GetCharacterMovement))))
                    (Variables|Default|SetgameOver true)
                    (bind _returnvalue_4 (UserInterface|CreateWidget "/Game/InfiniteMatrix/Blueprints/RestartButton.RestartButton_C"))
                    (bind _output_get_2 (Variables|Default|SetRestartButton_UI _returnvalue_4))
                    (UserInterface|Viewport|AddtoViewport _output_get_2 0)
                    (Variables|/Script/Engine.PlayerController|SetbShowMouseCursor (Game|GetPlayerController 0) true)))
                (:CastFailed
                  (Utilities|Casting|CastToEagle OtherActor)
                  (Transformation|DetachFromComponent (Variables|Default|GetCamera) "KeepWorld" "KeepWorld" "KeepWorld" true)
                  (Variables|Default|SetgameOver true)
                  (bind _returnvalue_5 (UserInterface|CreateWidget "/Game/InfiniteMatrix/Blueprints/RestartButton.RestartButton_C"))
                  (bind _output_get_3 (Variables|Default|SetRestartButton_UI _returnvalue_5))
                  (UserInterface|Viewport|AddtoViewport _output_get_3 0)
                  (Variables|/Script/Engine.PlayerController|SetbShowMouseCursor (Game|GetPlayerController 0) true))))))))))

(event EventBeginPlay
  (Variables|Default|Setscore 0)
  (bind _returnvalue (UserInterface|CreateWidget "/Game/InfiniteMatrix/Blueprints/Score.Score_C"))
  (UserInterface|Viewport|AddtoViewport _returnvalue 0))

(event EventTick
  (params (DeltaSeconds :type Float%20%28single-precision%29))
  (Development|PrintString (Utilities|String|ToString(Boolean) (Variables|Default|GetisSnapping)))
  (if (== (.z (Pawn|Components|CharacterMovement|GetLastUpdateVelocity (Variables|Character|GetCharacterMovement))) 0.0)
    (Variables|Default|SetcanMove true)
    (else
      (Variables|Default|SetcanMove false))))

(event Input|AxisEvents|InputAxisMoveForward
  (params (AxisValue :type Float%20%28single-precision%29))
  (bind _chicken (Variables|Default|GetChicken))
  (bind _chicken_2 (Variables|Default|GetChicken))
  (bind _chicken_3 (Variables|Default|GetChicken))
  (bind _currentlane (Variables|Default|GetcurrentLane))
  (bind _chicken_4 (Variables|Default|GetChicken))
  (bind _returnvalue (Transformation|GetWorldLocation _chicken_2))
  (bind _returnvalue_2 (Transformation|GetWorldLocation _chicken_3))
  (if (not (Variables|Default|GetgameOver))
    (if (and (> (Math|Float|Absolute(Float) AxisValue) 0.3) (Variables|Default|GetcanMove))
      (Utilities|IsValid _currentlane
        (:Is%20Valid
          (Character|LaunchCharacter (Math|Vector|MakeVector (* AxisValue (* (.x (Variables|/Script/Engine.BoxComponent|GetBoxExtent (Variables|/Game/InfiniteMatrix/Blueprints/BP_Lane.BP_Lane_C|GetCenterCheckCollisionBox2 _currentlane))) 5.0)) 0.0 (Variables|Default|GetjumpHeight)) true true))
        (:Is%20Not%20Valid
          (Character|LaunchCharacter (Math|Vector|MakeVector (* AxisValue (Variables|Default|GetjumpRange)) 0.0 (Variables|Default|GetjumpHeight)) true true)))
      (if (> AxisValue 0.3)
        (bind _newtrack_0 (Timeline|Timeline PlayFromStart)
          (:Update
            (Transformation|SetWorldRotation _chicken_4 (Math|Rotator|Lerp(Rotator) (Transformation|GetWorldRotation _chicken_4) "0.000000,-90.000000,0.000000" _newtrack_0 true) false false))
          (:Finished
            (if (> (Variables|Default|GetBackwardJumpsInARow) 0)
              (Variables|Default|SetBackwardJumpsInARow (- (Variables|Default|GetBackwardJumpsInARow) 1))
              (Development|PrintString "Subtrated 1 from BacwardJumpsInARow" false false)
              (Timeline|Timeline_6 PlayFromStart
                (:Finished
                  (Game|SpawnActorfromClass "/Game/InfiniteMatrix/Blueprints/Eagle.Eagle_C" (Math|Transform|MakeTransform (Math|Vector|MakeVector (+ (.x _returnvalue) 2e+03) (.y _returnvalue) 9e+01) "0.000000,180.000000,0.000000" "1.000000,1.000000,1.000000") "AlwaysSpawn" "MultiplyWithRoot" 0 0)
                  (Development|PrintString "Eagle spawned" false false)))
              (else
                (Timeline|Timeline_6 PlayFromStart)))))
        (else
          (bind _newtrack_0_2 (Timeline|Timeline_0 PlayFromStart)
            (:Update
              (Transformation|SetWorldRotation _chicken (Math|Rotator|Lerp(Rotator) (Transformation|GetWorldRotation _chicken) "0.000000,90.000000,0.000000" _newtrack_0_2 true) false false))
            (:Finished
              (Variables|Default|SetBackwardJumpsInARow (+ (Variables|Default|GetBackwardJumpsInARow) 1))
              (if (> (Variables|Default|GetBackwardJumpsInARow) 2)
                (Development|PrintString "Spawn Eagle")
                (Game|SpawnActorfromClass "/Game/InfiniteMatrix/Blueprints/Eagle.Eagle_C" (Math|Transform|MakeTransform (Math|Vector|MakeVector (+ (.x _returnvalue_2) 2e+03) (.y _returnvalue_2) 9e+01) "0.000000,180.000000,0.000000" "1.000000,1.000000,1.000000") "AlwaysSpawn" "MultiplyWithRoot" 0 0)
                (Development|PrintString "Eagle spawned" false false)
                (else
                  (Timeline|Timeline_6 PlayFromStart))))))))))

(event Input|AxisEvents|InputAxisMoveRight
  (params (AxisValue :type Float%20%28single-precision%29))
  (bind _chicken (Variables|Default|GetChicken))
  (bind _chicken_2 (Variables|Default|GetChicken))
  (bind _chicken_3 (Variables|Default|GetChicken))
  (bind _returnvalue (Transformation|GetWorldLocation _chicken))
  (if (not (Variables|Default|GetgameOver))
    (if (and (> (Math|Float|Absolute(Float) AxisValue) 0.3) (Variables|Default|GetcanMove))
      (Character|LaunchCharacter (Math|Vector|MakeVector 0.0 (* AxisValue (Variables|Default|GetjumpRange)) (Variables|Default|GetjumpHeight)) true true)
      (if (> AxisValue 0.3)
        (bind _newtrack_0 (Timeline|Timeline_1 PlayFromStart)
          (:Update
            (Transformation|SetWorldRotation _chicken_3 (Math|Rotator|Lerp(Rotator) (Transformation|GetWorldRotation _chicken_3) "0, 0, 0" _newtrack_0 true) false false))
          (:Finished
            (Timeline|Timeline_6 PlayFromStart
              (:Finished
                (Game|SpawnActorfromClass "/Game/InfiniteMatrix/Blueprints/Eagle.Eagle_C" (Math|Transform|MakeTransform (Math|Vector|MakeVector (+ (.x _returnvalue) 2e+03) (.y _returnvalue) 9e+01) "0.000000,180.000000,0.000000" "1.000000,1.000000,1.000000") "AlwaysSpawn" "MultiplyWithRoot" 0 0)
                (Development|PrintString "Eagle spawned" false false)))))
        (else
          (bind _newtrack_0_2 (Timeline|Timeline_2 PlayFromStart)
            (:Update
              (Transformation|SetWorldRotation _chicken_2 (Math|Rotator|Lerp(Rotator) (Transformation|GetWorldRotation _chicken_2) "0.000000,-180.000000,0.000000" _newtrack_0_2 true) false false))
            (:Finished
              (Timeline|Timeline_6 PlayFromStart))))))))

(fn ConstructionScript)

(fn SpawnEagle
  (bind _chicken (Variables|Default|GetChicken))
  (bind _returnvalue (Transformation|GetWorldLocation _chicken))
  (Game|SpawnActorfromClass "/Game/InfiniteMatrix/Blueprints/Eagle.Eagle_C" (Math|Transform|MakeTransform (Math|Vector|MakeVector (+ (.x _returnvalue) 2e+02) (.y _returnvalue) 1e+02) "0.000000,180.000000,0.000000" "1.000000,1.000000,1.000000") "Undefined" "MultiplyWithRoot" 0 0)
  (Development|PrintString "Eagle spawned" false false))