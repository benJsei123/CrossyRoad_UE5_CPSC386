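; Log is a moving log actor that a BP_Chicken can ride, driven by projectile movement.
; On BeginPlay it rolls InitialSpeed and MaxSpeed independently at random.
; Box overlaps toggle the chicken's IsOnLog flag as it enters and leaves.
; Overlapping another Log sets InitialSpeed just below that log's, intended to slow colliding logs, though it leaves current velocity and MaxSpeed untouched.
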(event OnComponentBeginOverlap(Box)
  (params (OverlappedComponent :type Primitive%20Component%20Object%20Reference) (OtherActor :type Actor%20Object%20Reference) (OtherComp :type Primitive%20Component%20Object%20Reference) (OtherBodyIndex :type Integer) (bFromSweep :type Boolean) (SweepResult :type Hit%20Result%20Structure%20%28by%20ref%29))
  ;[1 1 1] slow logs down as soon as they collide
  (bind _aslog (Utilities|Casting|CastToLog OtherActor)
    (:then
      (Variables|/Script/Engine.ProjectileMovementComponent|SetInitialSpeed (Variables|Default|GetProjectileMovement) (- (Variables|/Script/Engine.ProjectileMovementComponent|GetInitialSpeed (Variables|Log_C|GetProjectileMovement _aslog)) 2e+01)))
    (:CastFailed
      (bind _asbp_chicken (Utilities|Casting|CastToBP_Chicken OtherActor))
      (Variables|/Game/InfiniteMatrix/Blueprints/BP_Chicken.BP_Chicken_C|SetisOnLog _asbp_chicken true))))

(event OnComponentEndOverlap(Box)
  (params (OverlappedComponent :type Primitive%20Component%20Object%20Reference) (OtherActor :type Actor%20Object%20Reference) (OtherComp :type Primitive%20Component%20Object%20Reference) (OtherBodyIndex :type Integer))
  (bind _asbp_chicken (Utilities|Casting|CastToBP_Chicken OtherActor))
  (Variables|/Game/InfiniteMatrix/Blueprints/BP_Chicken.BP_Chicken_C|SetisOnLog _asbp_chicken false))

(event EventBeginPlay
  (bind _returnvalue (Math|Random|RandomFloatinRange 1e+02 4e+02))
  (bind _projectilemovement (Variables|Default|GetProjectileMovement))
  (Variables|/Script/Engine.ProjectileMovementComponent|SetInitialSpeed _projectilemovement _returnvalue)
  (Variables|/Script/Engine.ProjectileMovementComponent|SetMaxSpeed _projectilemovement _returnvalue))

(fn ConstructionScript)