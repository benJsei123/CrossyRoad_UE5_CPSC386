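; BP_LaneSpawner procedurally builds the BP_Lane track of grass, highway, river and railroad lanes for a chicken crossing game.
; On BeginPlay it clears existing lanes, then spawns initial groups, each lane chained to the newest lane's SpawnPoint.
; After four beginner grass groups, types are random without immediate repeats, and maximum group size grows with BP_Chicken's score.
; The last lane of each highway group uses an unmarked mesh.
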(event EventBeginPlay
  (CallFunction|BeginPlay))

(fn ConstructionScript)

(fn SpawnLane
  (params (SpawnLocation :type Vector) (StaticMesh :type Static%20Mesh%20Object%20Reference) (lane_type_index :type Integer))
  (bind _returnvalue (Game|SpawnActorfromClass "/Game/InfiniteMatrix/Blueprints/BP_Lane.BP_Lane_C" (Math|Transform|MakeTransform SpawnLocation "0, 0, 0" "1.000000,1.000000,1.000000") "Undefined" "MultiplyWithRoot" 0 (or (== lane_type_index 1) (== lane_type_index 4)) (== lane_type_index 2) (== lane_type_index 3) (== lane_type_index 0) 0))
  (Components|StaticMesh|SetStaticMesh (Variables|/Game/InfiniteMatrix/Blueprints/BP_Lane.BP_Lane_C|GetLane _returnvalue) StaticMesh)
  (bind _output_get (Variables|Default|SetNewestLane _returnvalue))
  (Variables|/Game/InfiniteMatrix/Blueprints/BP_Lane.BP_Lane_C|SetLaneSpawner _output_get self)
  (bind _result (Math|Integer|IncrementInt (Variables|Default|GetlanesSpawned))
    (:%20%20
      (bind _output_get_2 (Variables|Default|SetlanesSpawned _result))
      (Development|PrintString (Utilities|String|ToString(Text) (Utilities|Text|FormatText "\"                  Lanes spawned:    {N} at {x}\"" _output_get_2 (.X (Math|Vector2D|BreakVector2D (Math|Conversions|ToVector2D(Vector) SpawnLocation))))) false false "(R=1.000000,G=0.026376,B=0.191370,A=1.000000)" 5.0))))

(fn SpawnLaneatSpawnPoint
  (CallFunction|SpawnRandomLaneType self "0.000000,0.000000,10.000000"))

(fn SpawnInitialLanes
  (Utilities|FlowControl|Sequence
    (:then_0
      (bind _outactors (Actor|GetAllActorsOfClass "/Game/InfiniteMatrix/Blueprints/BP_Lane.BP_Lane_C"))
      (for _array_element _outactors
        (Actor|DestroyActor _array_element)))
    (:then_1
      (for _index (range 0 8)
        (Utilities|IsValid (Variables|Default|GetNewestLane)
          (:Is%20Valid
            (CallFunction|SpawnLaneatSpawnPoint))
          (:Is%20Not%20Valid
            (CallFunction|SpawnRandomLaneType "0.000000,0.000000,10.000000")))))))

(fn SpawnRandomLaneType
  (params (SpawnLocation :type Vector))
  (bind _newestlane (Variables|Default|GetNewestLane))
  (LocalVariables|Setnew%20Location SpawnLocation)
  (if (< (Variables|Default|GetbeginnerLanesSpawned) 4)
    (Variables|Default|SetbeginnerLanesSpawned (+ (Variables|Default|GetbeginnerLanesSpawned) 1))
    (Variables|Default|SetmeshTypeIndex 0)
    (else
      (bind _output_get (Variables|Default|SetmeshTypeIndex (Math|Random|RandomIntegerinRange 0 3) :!label _label))
      (if (== _output_get (Variables|Default|GetlastMeshTypeIndex))
        (goto _label)
        (else
          _))))
  ;[1 1 1] Increasing the difficulty based on the chicken's score
  (bind _outactors (Actor|GetAllActorsOfClass "/Game/InfiniteMatrix/Blueprints/BP_Chicken.BP_Chicken_C"))
  (for _array_element _outactors
    (bind _output_get_2 (Variables|Default|SetlaneLevelDifficulty (Math|Integer|Max(Integer) (/ (Variables|/Game/InfiniteMatrix/Blueprints/BP_Chicken.BP_Chicken_C|Getscore _array_element) 2) 2))))
  (Variables|Default|SetlastMeshTypeIndex (Variables|Default|GetmeshTypeIndex))
  (Variables|Default|SetmaxLanes (Math|Random|RandomIntegerinRange 1 _output_get_2))
  (Development|PrintString (Utilities|String|ToString(Text) (Utilities|Text|FormatText "\"Spawning {N} lanes of type {mesh}\"" (Math|Random|RandomIntegerinRange 1 _output_get_2) (Variables|Default|GetmeshTypeIndex))) false false "(R=0.000000,G=0.660000,B=1.000000,A=1.000000)" 2e+01)
  (for _index (range 1 (Variables|Default|GetmaxLanes))
    (LocalVariables|SetnewMesh (Utilities|Select :Index (Variables|Default|GetmeshTypeIndex) :Option%200 "/Game/InfiniteMatrix/Meshes/bordered_grass_onelane.bordered_grass_onelane" :Option%201 "/Game/InfiniteMatrix/Meshes/highway_marked_onelane.highway_marked_onelane" :Option%202 "/Game/InfiniteMatrix/Meshes/river_one_lane.river_one_lane" :Option%203 "/Game/InfiniteMatrix/Meshes/RR_one_lane.RR_one_lane"))
    (Utilities|IsValid _newestlane
      (:Is%20Valid
        (LocalVariables|Setnew%20Location (Transformation|GetWorldLocation (Variables|/Game/InfiniteMatrix/Blueprints/BP_Lane.BP_Lane_C|GetSpawnPoint _newestlane))))
      (:Is%20Not%20Valid
        _))
    (if (and (== 1 (Variables|Default|GetmeshTypeIndex)) (or (== (Variables|Default|GetmaxLanes) 1) (== (Variables|Default|GetmaxLanes) _index)))
      (LocalVariables|SetnewMesh "/Game/InfiniteMatrix/Meshes/highway_unmarked_onelane.highway_unmarked_onelane")
      (Development|PrintString "unmarked highway" false false "(R=0.063354,G=1.000000,B=0.152692,A=1.000000)" 5.0)
      (bind _output_get_3 (Variables|Default|Setextra_index_umarked_lane 4)))
    (CallFunction|SpawnLane (LocalVariables|Getnew%20Location) (LocalVariables|GetnewMesh) (Variables|Default|GetmeshTypeIndex))))

(fn BeginPlay
  (CallFunction|SpawnInitialLanes)
  (Development|PrintString "Initial Lanes Spawned" false false))