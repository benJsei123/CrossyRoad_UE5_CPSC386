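; One lane of an endless chicken-crossing game, configured by flags as highway, water, railroad or grass.
; On BeginPlay, looping random-interval timers spawn vehicles and police cars, logs, or trains preceded by blinking warning lights, while grass scatters tree/rock spawners.
; Side triggers destroy vehicles, logs and trains, and a chicken trigger requests another lane from LaneSpawner.
; The center trigger awards score on first visit, sets CurrentLane and timeline-snaps the chicken's X to mid-lane.
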(event OnComponentBeginOverlap(TriggerZone)
  (params (OverlappedComponent :type Primitive%20Component%20Object%20Reference) (OtherActor :type Actor%20Object%20Reference) (OtherComp :type Primitive%20Component%20Object%20Reference) (OtherBodyIndex :type Integer) (bFromSweep :type Boolean) (SweepResult :type Hit%20Result%20Structure%20%28by%20ref%29))
  (Utilities|Casting|CastToBP_Chicken OtherActor)
  (Default|SpawnLaneatSpawnPoint (Variables|Default|GetLaneSpawner)))

(event OnComponentBeginOverlap(RVehicleTrigger)
  (params (OverlappedComponent :type Primitive%20Component%20Object%20Reference) (OtherActor :type Actor%20Object%20Reference) (OtherComp :type Primitive%20Component%20Object%20Reference) (OtherBodyIndex :type Integer) (bFromSweep :type Boolean) (SweepResult :type Hit%20Result%20Structure%20%28by%20ref%29))
  (bind _asvehicle (Utilities|Casting|CastToVehicle OtherActor)
    (:then
      (Actor|DestroyActor _asvehicle))
    (:CastFailed
      (bind _aslog (Utilities|Casting|CastToLog OtherActor)
        (:then
          (Actor|DestroyActor _aslog))
        (:CastFailed
          (bind _astrain (Utilities|Casting|CastToTrain OtherActor))
          (Actor|DestroyActor _astrain))))))

(event OnComponentBeginOverlap(LVehicleTrigger)
  (params (OverlappedComponent :type Primitive%20Component%20Object%20Reference) (OtherActor :type Actor%20Object%20Reference) (OtherComp :type Primitive%20Component%20Object%20Reference) (OtherBodyIndex :type Integer) (bFromSweep :type Boolean) (SweepResult :type Hit%20Result%20Structure%20%28by%20ref%29))
  (bind _asvehicle (Utilities|Casting|CastToVehicle OtherActor)
    (:then
      (Actor|DestroyActor _asvehicle))
    (:CastFailed
      (bind _aslog (Utilities|Casting|CastToLog OtherActor)
        (:then
          (Actor|DestroyActor _aslog))
        (:CastFailed
          (bind _astrain (Utilities|Casting|CastToTrain OtherActor))
          (Actor|DestroyActor _astrain))))))

(event OnComponentBeginOverlap(CenterCheckCollisionBox2)
  (params (OverlappedComponent :type Primitive%20Component%20Object%20Reference) (OtherActor :type Actor%20Object%20Reference) (OtherComp :type Primitive%20Component%20Object%20Reference) (OtherBodyIndex :type Integer) (bFromSweep :type Boolean) (SweepResult :type Hit%20Result%20Structure%20%28by%20ref%29))
  (bind _box (Variables|Default|GetBox))
  (bind _returnvalue (Transformation|GetWorldLocation _box))
  (bind _returnvalue_2 (+ (.x _returnvalue) 0.0))
  (bind _asbp_chicken (Utilities|Casting|CastToBP_Chicken OtherActor))
  (if (== (Variables|Default|Getvisited) true)
    (Variables|/Game/InfiniteMatrix/Blueprints/BP_Chicken.BP_Chicken_C|SetcurrentLane _asbp_chicken self :!label _label)
    ;[1 1 1] snap the chicken to lane mid after each jump on new lane
    (if (== (Variables|/Game/InfiniteMatrix/Blueprints/BP_Chicken.BP_Chicken_C|GetisSnapping _asbp_chicken) false)
      (Variables|/Game/InfiniteMatrix/Blueprints/BP_Chicken.BP_Chicken_C|SetisSnapping _asbp_chicken true)
      (bind _newtrack_0 (Timeline|Timeline PlayFromStart)
        (:Update
          (if (not (== _returnvalue_2 (.x (Transformation|GetWorldLocation (Variables|/Script/Engine.Actor|GetRootComponent _asbp_chicken)))))
            (Transformation|SetWorldLocation (Variables|/Script/Engine.Actor|GetRootComponent _asbp_chicken) (Math|Vector|MakeVector (.x (Math|Vector|Lerp(Vector) (Math|Vector|MakeVector (.x (Transformation|GetWorldLocation (Variables|/Script/Engine.Actor|GetRootComponent _asbp_chicken))) 0.0 (+ (.z _returnvalue) 15.0)) (Math|Vector|MakeVector _returnvalue_2 0.0 0.0) _newtrack_0)) (.y (Transformation|GetWorldLocation (Variables|/Script/Engine.Actor|GetRootComponent _asbp_chicken))) (.z (Transformation|GetWorldLocation (Variables|/Script/Engine.Actor|GetRootComponent _asbp_chicken)))) false false)
            (Development|PrintString "Centering Chicken" false false)))
        (:Finished
          (Variables|/Game/InfiniteMatrix/Blueprints/BP_Chicken.BP_Chicken_C|SetisSnapping _asbp_chicken false))))
    (else
      (Variables|Default|Setvisited true)
      (bind _outactors (Actor|GetAllActorsOfClass "/Game/InfiniteMatrix/Blueprints/BP_Chicken.BP_Chicken_C"))
      (for _array_element _outactors
        (Variables|/Game/InfiniteMatrix/Blueprints/BP_Chicken.BP_Chicken_C|Setscore _array_element (+ (Variables|/Game/InfiniteMatrix/Blueprints/BP_Chicken.BP_Chicken_C|Getscore _array_element) 1))
        (goto _label)))))

(event OnComponentBeginOverlap(Box)
  (params (OverlappedComponent :type Primitive%20Component%20Object%20Reference) (OtherActor :type Actor%20Object%20Reference) (OtherComp :type Primitive%20Component%20Object%20Reference) (OtherBodyIndex :type Integer) (bFromSweep :type Boolean) (SweepResult :type Hit%20Result%20Structure%20%28by%20ref%29))
  (Utilities|Casting|CastToBP_Chicken OtherActor)
  (Development|PrintString "CHicken Hopped on lane"))

(event Custom|SpawnTrains
  ;[1 1 1] Spawning Trains
  (if (Math|Random|RandomBool)
    (Variables|/Game/InfiniteMatrix/Blueprints/railroad_crossing_light.railroad_crossing_light_C|SetisBlinking (stale EventBeginPlay _returnvalue) true)
    (Utilities|FlowControl|Delay 2.0)
    (if (Variables|Default|GetStartingCarLocation)
      (Game|SpawnActorfromClass "/Game/InfiniteMatrix/Blueprints/Train.Train_C" (Math|Transform|MakeTransform (Variables|Default|GetEndLocation) "0.000000,-90.000000,0.000000" "1.000000,1.000000,1.000000") "Undefined" "MultiplyWithRoot" 0 0)
      (else
        (Game|SpawnActorfromClass "/Game/InfiniteMatrix/Blueprints/Train.Train_C" (Math|Transform|MakeTransform (Variables|Default|GetStartLocation) "0.000000,90.000000,0.000000" "1.000000,1.000000,1.000000") "Undefined" "MultiplyWithRoot" 0 0)))))

(event Custom|SpawnVehicles
  ;[1 1 1] Comment
  (if (Math|Random|RandomBool)
    (switch int (Math|Random|RandomInteger 11)
      (:0
        (if (Variables|Default|GetleftToRight) :!label _label
          (Game|SpawnActorfromClass "/Game/InfiniteMatrix/Blueprints/Vehicle.Vehicle_C" (Math|Transform|MakeTransform (Variables|Default|GetEndLocation) "0.000000,-90.000000,0.000000" "1.000000,1.000000,1.000000") "Undefined" "MultiplyWithRoot" 0 0)
          (else
            (Game|SpawnActorfromClass "/Game/InfiniteMatrix/Blueprints/Vehicle.Vehicle_C" (Math|Transform|MakeTransform (Variables|Default|GetStartLocation) "0.000000,90.000000,0.000000" "1.000000,1.000000,1.000000") "Undefined" "MultiplyWithRoot" 0 0))))
      (:1
        (goto _label))
      (:2
        (goto _label))
      (:3
        (goto _label))
      (:4
        (goto _label))
      (:5
        (goto _label))
      (:6
        (goto _label))
      (:7
        (goto _label))
      (:8
        (if (Variables|Default|GetleftToRight) :!label _label_2
          (Game|SpawnActorfromClass "/Game/InfiniteMatrix/Blueprints/PoliceCar.PoliceCar_C" (Math|Transform|MakeTransform (Variables|Default|GetEndLocation) "0.000000,-90.000000,0.000000" "1.000000,1.000000,1.000000") "Undefined" "MultiplyWithRoot" 0 0)
          (else
            (Game|SpawnActorfromClass "/Game/InfiniteMatrix/Blueprints/PoliceCar.PoliceCar_C" (Math|Transform|MakeTransform (Variables|Default|GetStartLocation) "0.000000,90.000000,0.000000" "1.000000,1.000000,1.000000") "Undefined" "MultiplyWithRoot" 0 0))))
      (:9
        (goto _label_2))
      (:10
        (goto _label_2)))))

(event Custom|SpawnLogs
  ;[1 1 1] Spawning Log
  (if (Math|Random|RandomBool)
    (if (Variables|Default|GetStartingCarLocation)
      (Game|SpawnActorfromClass "/Game/InfiniteMatrix/Blueprints/Log.Log_C" (Math|Transform|MakeTransform (Variables|Default|GetEndLocation) "0.000000,-90.000000,0.000000" "1.000000,1.000000,1.000000") "Undefined" "MultiplyWithRoot" 0 0)
      (else
        (Game|SpawnActorfromClass "/Game/InfiniteMatrix/Blueprints/Log.Log_C" (Math|Transform|MakeTransform (Variables|Default|GetStartLocation) "0.000000,90.000000,0.000000" "1.000000,1.000000,1.000000") "Undefined" "MultiplyWithRoot" 0 0)))))

(event EventBeginPlay
  (Variables|Default|SetleftToRight (Math|Random|RandomBool))
  (Variables|Default|SetStartLocation (Transformation|GetWorldLocation (Variables|Default|GetStart)))
  (Variables|Default|SetEndLocation (Transformation|GetWorldLocation (Variables|Default|GetEnd)))
  ;[1 1 1] Different Actions fordifferent lane types
  (if (Variables|Default|GetisHighway)
    ;[1 1 1] Comment
    (Variables|Default|SetStartingCarLocation (Math|Random|RandomBool))
    (Utilities|Time|SetTimerbyEvent (delegate Custom|SpawnVehicles) (Math|Random|RandomFloatinRange 2.0 3.0) true)
    (elif (Variables|Default|GetisWater)
      ;[1 1 1] Spawning Log
      (Variables|Default|SetStartingCarLocation (Math|Random|RandomBool))
      (Utilities|Time|SetTimerbyEvent (delegate Custom|SpawnLogs) (Math|Random|RandomFloatinRange 1.0 2.0) true)
      (elif (Variables|Default|GetisRailroad)
        (bind _returnvalue (Game|SpawnActorfromClass "/Game/InfiniteMatrix/Blueprints/railroad_crossing_light.railroad_crossing_light_C" (Math|Transform|MakeTransform (Transformation|GetWorldLocation (Variables|Debug|GetStaticMeshComponent)) "0.000000,90.000000,0.000000" "5.000000,5.000000,5.000000") "Undefined" "MultiplyWithRoot" 0 0))
        ;[1 1 1] Spawning Trains
        (Variables|Default|SetStartingCarLocation (Math|Random|RandomBool))
        (Utilities|Time|SetTimerbyEvent (delegate Custom|SpawnTrains) (Math|Random|RandomFloatinRange 8.0 2e+01) true)
        (elif (Variables|Default|GetisGrass)
          ;[1 1 1] Spawnig Rocks and trees
          (Variables|Default|SetStartLocation (Transformation|GetWorldLocation (Variables|Default|GetStart)))
          (Variables|Default|SetEndLocation (Transformation|GetWorldLocation (Variables|Default|GetEnd)))
          (for _index (range 0 (Math|Float|Truncate (/ (Math|Vector|Distance(Vector) (Variables|Default|GetStartLocation) (Variables|Default|GetEndLocation)) 82.0)))
            (if (>= (Math|Random|RandomFloat) 0.7)
              (Game|SpawnActorfromClass "/Game/InfiniteMatrix/Blueprints/TreeRockSpawner.TreeRockSpawner_C" (Math|Transform|MakeTransform (Math|Vector|MakeVector (.x (Variables|Default|GetStartLocation)) (+ (* _index 90) (.y (Variables|Default|GetStartLocation))) (.z (Variables|Default|GetStartLocation))) "0, 0, 0" "1.000000,1.000000,1.000000") "Undefined" "MultiplyWithRoot" 0 0))))))))

(event EventTick
  (params (DeltaSeconds :type Float%20%28single-precision%29)))

(fn ConstructionScript)